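; Table actor that procedurally seats chairs around its rim at construction; the event graph is empty.
; The construction script spaces Chair child actors along the TableRim spline by seat count, tagging each with an indexed chair name.
; Each chair mesh's rotation blends the spline's orientation partly toward an offset look-at of the local origin, roughly facing the table center.
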(event EventBeginPlay)

(event Collision|EventActorBeginOverlap
  (params (OtherActor :type Actor%20Object%20Reference)))

(event EventTick
  (params (DeltaSeconds :type Float%20%28single-precision%29)))

(fn ConstructionScript
  (bind _numseats (Variables|Default|GetnumSeats))
  (bind _returnvalue (Class|KismetSystemLibrary|MakeLiteralInteger _numseats))
  ;[1 1 1] Place chairs around the table
  (for _index (range 0 _returnvalue)
    (bind _returnvalue_2 (AddComponent|AddChildActorComponent false (Spline|GetTransformatDistanceAlongSpline (Variables|Default|GettableRim) (* _index (/ (Spline|GetSplineLength (Variables|Default|GettableRim)) (Math|Conversions|ToFloat(Integer) _returnvalue))) "Local" false)))
    (ChildActorComponent|SetChildActorClass _returnvalue_2 "/Game/Blueprints/chair.chair_C")
    ;;[1 1 1] Set chair number
    (bind _aschair (Utilities|Casting|CastTochair (Variables|/Script/Engine.ChildActorComponent|GetChildActor _returnvalue_2)))
    (Variables|/Script/Engine.Actor|SetTags _aschair (Utilities|Array|MakeArray (Utilities|String|StringToName (Utilities|String|Append (Utilities|String|MakeLiteralString "chair") (Utilities|String|ToString(Integer) _index)))))
    ;;[1 1 1] Kinda rotate chairs to face center of table
    (Transformation|SetRelativeRotation (Variables|/Game/Blueprints/chair.chair_C|GetchairMesh _aschair) (Math|Rotator|CombineRotators (Math|Rotator|Lerp(Rotator) (.Rotation (Math|Transform|BreakTransform (Spline|GetTransformatDistanceAlongSpline (Variables|Default|GettableRim) (* _index (/ (Spline|GetSplineLength (Variables|Default|GettableRim)) (Math|Conversions|ToFloat(Integer) _returnvalue))) "Local" false))) (Math|Rotator|CombineRotators (Math|Rotator|FindLookatRotation (.Location (Math|Transform|BreakTransform (Spline|GetTransformatDistanceAlongSpline (Variables|Default|GettableRim) (* _index (/ (Spline|GetSplineLength (Variables|Default|GettableRim)) (Math|Conversions|ToFloat(Integer) _returnvalue))) "Local" false))) (Math|Vector|MakeVector 0.0 0.0 0.0)) "0,-90.000000, 0") 0.3 true) (Class|KismetMathLibrary|NegateRotator (.Rotation (Math|Transform|BreakTransform (Spline|GetTransformatDistanceAlongSpline (Variables|Default|GettableRim) (* _index (/ (Spline|GetSplineLength (Variables|Default|GettableRim)) (Math|Conversions|ToFloat(Integer) _returnvalue))) "Local" false))))) false false)))