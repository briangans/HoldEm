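; A playing card Blueprint that holds a value made of a tier and a suit and displays it as text.
; SetValue stores the value, joins the tier and suit enum names into one string, and writes it to both TextRender components.
; BeginPlay only prints a debug message, and the construction script is empty.
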(event Custom|SetValue
  (params (value :type Card%20Structure))
  (bind _output_get (Variables|Default|Setvalue value))
  (Rendering|Components|TextRender|SetText (Variables|Default|GetTextRender) (Utilities|Text|ToText(String) (Utilities|String|Append (Utilities|String|EnumtoString (.tier (Utilities|Struct|Breakcard _output_get))) " 
" (Utilities|String|EnumtoString (.suit (Utilities|Struct|Breakcard _output_get))))))
  (Rendering|Components|TextRender|SetText (Variables|Default|GetTextRender1) (Utilities|Text|ToText(String) (Utilities|String|Append (Utilities|String|EnumtoString (.tier (Utilities|Struct|Breakcard _output_get))) " 
" (Utilities|String|EnumtoString (.suit (Utilities|Struct|Breakcard _output_get)))))))

(event EventBeginPlay
  (Development|PrintString "I exist!"))

(fn ConstructionScript)