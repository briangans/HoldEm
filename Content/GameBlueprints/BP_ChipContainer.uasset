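; BP_ChipContainer is an actor that holds a value as a pile of poker chip meshes, with a flag widget displaying that value.
; SetValue rebuilds the chips, while GiveValue hands existing meshes to another container by reattaching them in world space.
; The receiving container enables Tick to lerp incoming chips into place over a quarter second, using a Gate and DoOnce to switch Tick off when none are moving.
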(event Custom|ReceiveValue
  (params (addValue :type Integer))
  ;[1 1 1] Receive value and chips from another container
  (Variables|Default|Setvalue (+ addValue (Variables|Default|Getvalue)))
  (Utilities|UpdateUIFlagValue
    (:out
      (Actor|Tick|SetActorTickEnabled true) ; Turn on tick to move chips
    )))

(event Custom|ClearCollection
  (Utilities|Array|Clear (Variables|Default|GetchipArray))
  (Development|PrintString "CC: Clear, is this even used?" true true "(R=0.000000,G=0.660000,B=1.000000,A=1.000000)" 999.0))

(event Custom|SetValue
  (params (value :type Integer))
  (bind _chiparray (Variables|Default|GetchipArray))
  ;[1 1 1] Set chip value for this container
  (bind _output_get (Variables|Default|Setvalue value))
  (Utilities|UpdateUIFlagValue
    (:out
      ;;[1 1 1] Delete chip actors
      (for _array_element _chiparray
        (Components|DestroyComponent (.staticmeshcomp _array_element)))
      (Utilities|Array|Clear _chiparray)
      ;;[1 1 1] Create chips
      (for _index (range 0 (- (/ _output_get (Variables|Default|GetindividualChipValue)) 1))
        (bind _returnvalue (AddComponent|AddStaticMeshComponent true (Utilities|GetRTforNewChipMesh (Variables|Default|GetchipArray))))
        (Components|StaticMesh|SetStaticMesh _returnvalue "/Game/MeshAssets/chip/SM_PokerChip.SM_PokerChip")
        (Utilities|Array|AddUnique (Variables|Default|GetchipArray) (Utilities|Struct|MakeSchip _returnvalue false))
        (Transformation|AttachComponentToComponent _returnvalue (Variables|Default|GetDefaultSceneRoot) "None" "KeepRelative" "KeepRelative" "KeepRelative" false)))))

(event Custom|GiveValue
  (params (GiveValue :type Integer) (toChipContainer :type BP%20Chip%20Container%20Object%20Reference%20%28by%20ref%29))
  (bind _chiparray (Variables|Default|GetchipArray))
  (bind _chiparray_2 (Variables|Default|GetchipArray))
  (bind _returnvalue (Utilities|Array|LastIndex _chiparray_2))
  (bind _output (Utilities|Array|Get(acopy) _chiparray_2 _returnvalue))
  ;[1 1 1] Give chips and value to another chip container
  (Variables|Default|Setvalue (- (Variables|Default|Getvalue) GiveValue))
  (Utilities|UpdateUIFlagValue
    (:out
      (for _index (range 0 (- (/ GiveValue (Variables|Default|GetindividualChipValue)) 1))
        (Transformation|AttachComponentToComponent (.staticmeshcomp _output) (Variables|BP_ChipContainer_C|GetDefaultSceneRoot toChipContainer) "None" "KeepWorld" "KeepWorld" "KeepWorld" false)
        (Utilities|Array|AddUnique (Variables|BP_ChipContainer_C|GetchipArray toChipContainer) (Utilities|Struct|MakeSchip (.staticmeshcomp _output) true (Transformation|GetRelativeTransform (.staticmeshcomp _output)) (Utilities|GetRTforNewChipMesh (Variables|BP_ChipContainer_C|GetchipArray toChipContainer))))
        (Utilities|Array|RemoveIndex _chiparray (Utilities|Array|LastIndex _chiparray)))
      (CallFunction|ReceiveValue toChipContainer GiveValue))))

(event EventBeginPlay
  (Utilities|UpdateUIFlagValue))

(event EventTick
  (params (DeltaSeconds :type Float%20%28single-precision%29))
  (bind _chiparray (Variables|Default|GetchipArray))
  ;[1 1 1] Chip motion
  (Utilities|FlowControl|Sequence
    (:then_0
      (goto _label_2 Open))
    (:then_1
      (goto _label Reset))
    (:then_2
      (for (_array_element _array_index) _chiparray
        (if (and (.moving _array_element) (not (Class|ActorComponent|IsBeingDestroyed (.staticmeshcomp _array_element))))
          (Utilities|FlowControl|Sequence
            (:then_0
              (Utilities|FlowControl|DoOnce false :!label _label
                (:Completed
                  (goto _label_2 Close))))
            (:then_1
              (|SetBy-RefVar (Utilities|Array|Get(acopy) _chiparray _array_index) (Utilities|Struct|MakeSchip (.staticmeshcomp _array_element) (< (* (+ (.movetimeelapsed _array_element) DeltaSeconds) 4.0) 1.0) (.starttransform _array_element) (.endtransform _array_element) (+ (.movetimeelapsed _array_element) DeltaSeconds)))
              (if (< (* (+ (.movetimeelapsed _array_element) DeltaSeconds) 4.0) 1.0)
                (Transformation|SetRelativeTransform (.staticmeshcomp _array_element) (Math|Transform|Lerp(Transform) (.starttransform _array_element) (.endtransform _array_element) (* (+ (.movetimeelapsed _array_element) DeltaSeconds) 4.0)) false false)
                (else
                  (Transformation|SetRelativeTransform (.staticmeshcomp _array_element) (.endtransform _array_element) false false) ; Snap to destination
                ))))))
      (Utilities|FlowControl|Gate true :!label _label_2
        (:Exit
          (Actor|Tick|SetActorTickEnabled false) ; Turn off tick if no chips need moving
        )))))

(fn ConstructionScript)

(fn UpdateUIFlagName
  (params (text :type Text))
  (bind _asflag_chip_container (Utilities|Casting|CastToflag-chipContainer (UserInterface|GetUserWidgetObject (Variables|Default|GetWidget%20flag))))
  (Default|SetName _asflag_chip_container text))