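; BP_DealerButton is the dealer button actor, which moves to a given transform over a given duration.
; SetDestination records the current transform as the start, stores the target and duration, and flags the button as travelling.
; While travelling, Tick linearly interpolates the whole transform by elapsed time without sweeping, then snaps to the exact target and stops.
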(event Custom|SetDestination
  (params (transform :type Transform) (time :type Float%20%28double-precision%29))
  (Variables|Default|Settravelling true)
  (Variables|Default|SetmovementDuration time)
  (Variables|Default|SetmovementElapsed 0.0)
  (Variables|Default|SetendTransform transform)
  (Variables|Default|SetstartTransform (Transformation|GetActorTransform)))

(event EventTick
  (params (DeltaSeconds :type Float%20%28single-precision%29))
  (if (Variables|Default|Gettravelling)
    (Transformation|SetActorTransform (Math|Transform|Lerp(Transform) (Variables|Default|GetstartTransform) (Variables|Default|GetendTransform) (/ (Variables|Default|GetmovementElapsed) (Variables|Default|GetmovementDuration))))
    (Variables|Default|SetmovementElapsed (+ (Variables|Default|GetmovementElapsed) DeltaSeconds))
    (if (>= (Variables|Default|GetmovementElapsed) (Variables|Default|GetmovementDuration))
      (Variables|Default|Settravelling false)
      (Transformation|SetActorTransform (Variables|Default|GetendTransform)))))

(fn ConstructionScript)