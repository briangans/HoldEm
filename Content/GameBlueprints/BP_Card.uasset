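; BP_Card is a playing card actor for a Hold'em game that shows its tier and suit and moves around the table.
; Public and private set-value events share one path that writes two text renders and a flag-card widget, retrying after a delay until the widget exists.
; SetDestination starts a timed move, which Tick interpolates from the current transform to the target and snaps on completion.
; A helper sends debug text to the HUD.
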(event Custom|PublicSetValue
  (params (value :type Scard%20Structure))
  (bind _widget_flag (Variables|Default|GetWidget%20flag))
  ;[1 1 1] Set Card Value (replace later with texture manip)
  (Variables|Default|Setvalue value)
  (Variables|Default|Setpublic (.public (Utilities|Struct|BreakScard (Variables|Default|Getvalue))))
  (Rendering|Components|TextRender|SetText (Variables|Default|GetTextRender) (Utilities|Text|ToText(String) (Utilities|String|Append (Utilities|String|EnumtoString (.tier (Utilities|Struct|BreakScard (Variables|Default|Getvalue)))) " 
" (Utilities|String|EnumtoString (.suit (Utilities|Struct|BreakScard (Variables|Default|Getvalue)))))))
  (Rendering|Components|TextRender|SetText (Variables|Default|GetTextRender1) (Utilities|Text|ToText(String) (Utilities|String|Append (Utilities|String|EnumtoString (.tier (Utilities|Struct|BreakScard (Variables|Default|Getvalue)))) " 
" (Utilities|String|EnumtoString (.suit (Utilities|Struct|BreakScard (Variables|Default|Getvalue)))))))
  ;[1 1 1] Set data on widget
  (Rendering|SetVisibility _widget_flag true false)
  (bind _asflag_card (Utilities|Casting|CastToflag-card (UserInterface|GetUserWidgetObject _widget_flag) :!label _label)
    (:then
      (Default|SetValue _asflag_card (.tier (Utilities|Struct|BreakScard (Variables|Default|Getvalue))) (.suit (Utilities|Struct|BreakScard (Variables|Default|Getvalue)))))
    (:CastFailed
      (Utilities|FlowControl|Delay 0.2)
      (goto _label))))

(event Custom|PrivateSetValue
  (params (value :type Scard%20Structure))
  (bind _widget_flag (Variables|Default|GetWidget%20flag))
  ;[1 1 1] Set Card Value (replace later with texture manip)
  (Variables|Default|Setvalue value)
  (Variables|Default|Setpublic (.public (Utilities|Struct|BreakScard (Variables|Default|Getvalue))))
  (Rendering|Components|TextRender|SetText (Variables|Default|GetTextRender) (Utilities|Text|ToText(String) (Utilities|String|Append (Utilities|String|EnumtoString (.tier (Utilities|Struct|BreakScard (Variables|Default|Getvalue)))) " 
" (Utilities|String|EnumtoString (.suit (Utilities|Struct|BreakScard (Variables|Default|Getvalue)))))))
  (Rendering|Components|TextRender|SetText (Variables|Default|GetTextRender1) (Utilities|Text|ToText(String) (Utilities|String|Append (Utilities|String|EnumtoString (.tier (Utilities|Struct|BreakScard (Variables|Default|Getvalue)))) " 
" (Utilities|String|EnumtoString (.suit (Utilities|Struct|BreakScard (Variables|Default|Getvalue)))))))
  ;[1 1 1] Set data on widget
  (Rendering|SetVisibility _widget_flag true false)
  (bind _asflag_card (Utilities|Casting|CastToflag-card (UserInterface|GetUserWidgetObject _widget_flag) :!label _label)
    (:then
      (Default|SetValue _asflag_card (.tier (Utilities|Struct|BreakScard (Variables|Default|Getvalue))) (.suit (Utilities|Struct|BreakScard (Variables|Default|Getvalue)))))
    (:CastFailed
      (Utilities|FlowControl|Delay 0.2)
      (goto _label))))

(event Custom|SetDestination
  (params (transform :type Transform) (time :type Float%20%28double-precision%29))
  ;[1 1 1] Card Movement
  (Variables|cardMovement|Settravelling true)
  (Variables|cardMovement|SetmovementDuration time)
  (Variables|cardMovement|SetmovementElapsed 0.0)
  (Variables|cardMovement|SetendTransform transform)
  (Variables|cardMovement|SetstartTransform (Transformation|GetActorTransform)))

(event EventTick
  (params (DeltaSeconds :type Float%20%28single-precision%29))
  ;[1 1 1] Card Movement
  (if (Variables|cardMovement|Gettravelling)
    (Transformation|SetActorTransform (Math|Transform|Lerp(Transform) (Variables|cardMovement|GetstartTransform) (Variables|cardMovement|GetendTransform) (/ (Variables|cardMovement|GetmovementElapsed) (Variables|cardMovement|GetmovementDuration))))
    (Variables|cardMovement|SetmovementElapsed (+ (Variables|cardMovement|GetmovementElapsed) DeltaSeconds))
    (if (>= (Variables|cardMovement|GetmovementElapsed) (Variables|cardMovement|GetmovementDuration))
      (Variables|cardMovement|Settravelling false)
      (Transformation|SetActorTransform (Variables|cardMovement|GetendTransform)))))

(fn ConstructionScript)

(fn LocalDebug
  (params (string :type String))
  (bind _asplayer_controller_hold_em (Utilities|Casting|CastToPlayerControllerHoldEm (Game|GetPlayerController 0)))
  (bind _ashud_hold_em (Utilities|Casting|CastToHudHoldEm (HUD|GetHUD _asplayer_controller_hold_em)))
  (Default|SetDebugText _ashud_hold_em string))