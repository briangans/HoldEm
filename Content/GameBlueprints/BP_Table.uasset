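; BP_Table is a game table with configurable seating and a chip pot, whose container UI name it sets to "Pot" through a custom event.
; Its construction script spawns BP_Chair child actors evenly spaced along the TableRim spline and tags each with its seat index.
; Each chair mesh is partly rotated toward the world origin, which faces the table center only when the table sits there.
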(event Custom|SetChipContainerPotName
  (bind _aschip_container (Utilities|Casting|CastToBP_ChipContainer (Variables|/Script/Engine.ChildActorComponent|GetChildActor (Variables|Default|GetchipContainerPot))))
  (Default|UpdateUIFlagName _aschip_container "Pot"))

(fn ConstructionScript
  (bind _numseats (Variables|Default|GetnumSeats))
  ;[1 1 1] Place chairs around the table
  (for _index (range 0 (- _numseats 1))
    (bind _returnvalue (AddComponent|AddChildActorComponent false (Spline|GetTransformatDistanceAlongSpline (Variables|Default|GettableRim) (* _index (/ (Spline|GetSplineLength (Variables|Default|GettableRim)) (Math|Conversions|ToFloat(Integer) _numseats))) "Local" false)))
    (ChildActorComponent|SetChildActorClass _returnvalue "/Game/GameBlueprints/BP_Chair.BP_Chair_C")
    ;;[1 1 1] Set chair number tag
    (bind _aschair (Utilities|Casting|CastToBP_Chair (Variables|/Script/Engine.ChildActorComponent|GetChildActor _returnvalue)))
    (Variables|/Script/Engine.Actor|SetTags _aschair (Utilities|Array|MakeArray (Utilities|String|StringToName (Utilities|String|Append (Utilities|String|MakeLiteralString "chair") (Utilities|String|ToString(Integer) _index)))))
    ;;[1 1 1] Kinda rotate chairs to face center of table
    (Transformation|SetWorldRotation (Variables|/Game/GameBlueprints/BP_Chair.BP_Chair_C|GetchairMesh _aschair) (Math|Rotator|Lerp(Rotator) (Transformation|GetWorldRotation (Variables|/Game/GameBlueprints/BP_Chair.BP_Chair_C|GetchairMesh _aschair)) (Math|Rotator|FindLookatRotation (Transformation|GetWorldLocation (Variables|/Game/GameBlueprints/BP_Chair.BP_Chair_C|GetchairMesh _aschair)) (Math|Vector|MakeVector 0.0 0.0 0.0)) 0.3 true) false false)))