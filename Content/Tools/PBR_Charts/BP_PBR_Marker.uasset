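; BP_PBR_Marker is a labeled marker actor for PBR charts, placed along a value axis according to its Color.
; The construction script passes Color to the line via custom primitive data, scales the Scene component by Offset and fills five text renders with one label.
; It then snaps the actor to a fixed world X, deriving Y from the color's HSV value through an inverted 2.2 power curve.
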(event EventBeginPlay)

(event Collision|EventActorBeginOverlap
  (params (OtherActor :type Actor%20Object%20Reference)))

(event EventTick
  (params (DeltaSeconds :type Float%20%28single-precision%29)))

(fn ConstructionScript
  (bind _offset (Variables|Default|GetOffset))
  (bind _textrender (Variables|Default|GetTextRender))
  (bind _color (Variables|Default|GetColor))
  (bind _returnvalue (Math|Conversions|ToVector(LinearColor) _color))
  (Rendering|Material|SetDefaultCustomPrimitiveDataVector4 (Variables|Default|GetLIne) 0 (Math|Vector4|MakeVector4 (.x _returnvalue) (.y _returnvalue) (.z _returnvalue) 1.0))
  (Transformation|SetRelativeScale3D (Variables|Default|GetScene) (Math|Vector|MakeVector _offset 0.05 0.05))
  (Transformation|SetRelativeLocation _textrender (Math|Vector|MakeVector (+ (* _offset 1e+02) 5.0) 0.0 6.0) false false)
  (Rendering|Components|TextRender|SetText _textrender (Variables|Default|GetText))
  (Transformation|SetActorLocation self (Math|Vector|MakeVector -5e+02 (* (- (- 1.0 (Math|Float|Power (- 1.0 (.V (Math|Color|RGBtoHSV(LinearColor) _color))) 2.2)) 0.5) -1e+03) 0.0) false false))